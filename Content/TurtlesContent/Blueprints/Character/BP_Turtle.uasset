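; BP_Turtle is a turtle character Blueprint that defines what the turtle does on reaching its finish spot.
; OnFinish plays the finish montage, then waits for that montage's default blend-out time rather than its length.
; It then sets the capsule to ignore all collision, turns the mesh into a physics-simulated body, and sets a lifespan so the actor is later destroyed.
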(event `OnFinish`
  (bind _am_finish (`self.AM_Finish`))
  (bind _mesh (`self.Mesh`))
  ;[1 1 1] Actions to do when reaching finish spot
  (`self.PlayAnimMontage` _am_finish)
  (`KismetSystemLibrary.Delay` (`AnimMontage.GetDefaultBlendOutTime` _am_finish))
  (`PrimitiveComponent.SetCollisionResponseToAllChannels` (`self.CapsuleComponent`) "ECR_Ignore")
  (`PrimitiveComponent.SetCollisionEnabled` _mesh "QueryAndPhysics")
  (`PrimitiveComponent.SetSimulatePhysics` _mesh true)
  (`self.SetLifeSpan` (`self.Lifespan`)))

(fn `UserConstructionScript`)