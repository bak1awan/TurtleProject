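; BP_Finish is the finish point actor that turtles reach in the game.
; When its Box is overlapped by a BP_Turtle, it calls that turtle's OnFinish event and plays finish effects.
; The effects are a sound at FinishSpot and a particle emitter spawned at each of four corner components, which BeginPlay gathers into an array.
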(event `self.ReceiveBeginPlay`
  ;[1 1 1] Store all the corners
  (set `self.Corners` (`|MakeArray` (`self.Corner1`) (`self.Corner2`) (`self.Corner3`) (`self.Corner4`))))

(event `self.Box.OnComponentBeginOverlap`
  (params (OverlappedComponent :type "PrimitiveComponent Object Reference") (OtherActor :type "Actor Object Reference") (OtherComp :type "PrimitiveComponent Object Reference") (OtherBodyIndex :type Integer) (bFromSweep :type Boolean) (SweepResult :type "HitResult Structure (by ref)"))
  ;[1 1 1] When turtle gets to the finish point - call its OnFinish event and play effects
  (bind _asbp_turtle (cast `/Game/TurtlesContent/Blueprints/Character/BP_Turtle` OtherActor))
  (`/Game/TurtlesContent/Blueprints/Character/BP_Turtle.OnFinish` _asbp_turtle)
  (`self.PlayEffectsOnFinish`))

(event `PlayEffectsOnFinish`
  ;[1 1 1] Plays sound and VFX when turtle gets to the finish
  (`GameplayStatics.PlaySoundAtLocation` (`self.FInishSound`) (`SceneComponent.K2_GetComponentLocation` (`self.FinishSpot`)) (struct) 1.0 1.0 0.0 null null null)
  (for _array_element (`self.Corners`)
    (bind (_returnvalue_location _returnvalue_rotation _returnvalue_scale) (`KismetMathLibrary.BreakTransform` (`SceneComponent.K2_GetComponentToWorld` _array_element)))
    (`GameplayStatics.SpawnEmitterAtLocation` (`self.FinishEffect`) _returnvalue_location _returnvalue_rotation _returnvalue_scale)))

(fn `UserConstructionScript`)