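; An interactable button that spawns turtles from every BP_Nest sharing its tag, gathered at BeginPlay.
; When the third-person character interacts, a timeline lerps the mesh down and is reversed after a one-second delay.
; The timeline's Finished output calls SpawnTurtle on each nest and resets the DoOnce that blocks repeat presses.
; A box overlap shows and removes the interact widget as the character enters and leaves.
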(event `self.ReceiveBeginPlay`
  ;[1 1 1] Store all the nests connected to the button
  (bind _outactors (`GameplayStatics.GetAllActorsOfClassWithTag` "/Game/TurtlesContent/Blueprints/Environment/BP_Nest.BP_Nest_C" (`self.TagName`)))
  (set `self.Nests` _outactors)
  ;[1 1 1] And set button pressed/normal location
  (bind _output_get (set `self.NormalLocation` (`SceneComponent.K2_GetComponentLocation` (`self.ButtonMesh`))))
  (set `self.PressedLocation` (- _output_get (0.0 0.0 8.0))))

(event `/Game/TurtlesContent/Blueprints/InteractInterface.Interact`
  (params (Interactor :type "Character Object Reference"))
  ;[1 1 1] On Event interact - change button location and spawn turtle
  (cast `/Game/TurtlesContent/Blueprints/Character/BP_ThirdPersonCharacter` Interactor)
  (`/Engine/EditorBlueprintResources/StandardMacros.DoOnce` false :!label _label
    (:`Completed`
      (`|ExecutionSequence`
        (:`then_0`
          (bind (_direction _alpha) (`Timeline|Alpha` :!label _label_2)
            (:`Update`
              (`SceneComponent.K2_SetWorldLocation` (`self.ButtonMesh`) (`KismetMathLibrary.VLerp` (`self.NormalLocation`) (`self.PressedLocation`) _alpha) false false))
            (:`Finished`
              (for _array_element (`self.Nests`)
                (bind _asbp_nest (cast `/Game/TurtlesContent/Blueprints/Environment/BP_Nest` _array_element))
                (`/Game/TurtlesContent/Blueprints/Environment/BP_Nest.SpawnTurtle` _asbp_nest)
                (goto _label :!via `Reset`)))))
        (:`then_1`
          (`KismetSystemLibrary.Delay` 1.0)
          (goto _label_2 :!via `Reverse`))))))

(event `self.Box.OnComponentBeginOverlap`
  (params (OverlappedComponent :type "PrimitiveComponent Object Reference") (OtherActor :type "Actor Object Reference") (OtherComp :type "PrimitiveComponent Object Reference") (OtherBodyIndex :type Integer) (bFromSweep :type Boolean) (SweepResult :type "HitResult Structure (by ref)"))
  ;[1 1 1] Add and remove widget when player get close to the button
  (cast `/Game/TurtlesContent/Blueprints/Character/BP_ThirdPersonCharacter` OtherActor)
  (bind _returnvalue (`|CreateWidget` "/Game/TurtlesContent/Blueprints/BP_InteractWIdget.BP_InteractWIdget_C"))
  (`UserWidget.AddToViewport` _returnvalue 0))

(event `self.Box.OnComponentEndOverlap`
  (params (OverlappedComponent :type "PrimitiveComponent Object Reference") (OtherActor :type "Actor Object Reference") (OtherComp :type "PrimitiveComponent Object Reference") (OtherBodyIndex :type Integer))
  ;[1 1 1] Add and remove widget when player get close to the button
  (cast `/Game/TurtlesContent/Blueprints/Character/BP_ThirdPersonCharacter` OtherActor)
  (`Widget.RemoveFromParent` (stale `self.Box.OnComponentBeginOverlap` _returnvalue)))

(fn `UserConstructionScript`)