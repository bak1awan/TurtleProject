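; BP_Nest is a spawn point that creates turtles heading toward a finish.
; On BeginPlay it finds BP_Finish actors by tag, caches the finish spot as the aim location and stores its four corner components.
; SpawnTurtle spawns a BP_Turtle at the nest, passing it the aim and nest locations and a behavior tree.
; Each spawn plays creature and nest sounds, plus particle emitters at the four corners.
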(event `self.ReceiveBeginPlay`
  ;[1 1 1] Event there is an array as the output pin in Get All Actors of Class with Tag function our Nest could be connected only to one Finish point
  (bind _outactors (`GameplayStatics.GetAllActorsOfClassWithTag` "/Game/TurtlesContent/Blueprints/Environment/BP_Finish.BP_Finish_C" (`self.TagName`)))
  (bind _output_get (set `self.FinishActors` _outactors))
  (for _array_element _output_get
    (bind _asbp_finish (cast `/Game/TurtlesContent/Blueprints/Environment/BP_Finish` _array_element))
    (set `self.AimLocation` (`SceneComponent.K2_GetComponentLocation` (`/Game/TurtlesContent/Blueprints/Environment/BP_Finish.FinishSpot` _asbp_finish)))
    ;[1 1 1] Store all the corners into the variable
    (set `self.Corners` (`|MakeArray` (`self.Corner1`) (`self.Corner2`) (`self.Corner3`) (`self.Corner4`)))))

(event `SpawnTurtle`
  ;[1 1 1] Spawn Turtle
  (bind _returnvalue (`|SpawnActorFromClass` "/Game/TurtlesContent/Blueprints/Character/BP_Turtle.BP_Turtle_C" (`SceneComponent.K2_GetComponentToWorld` (`self.Scene`)) "AlwaysSpawn" "OverrideRootScale" null null))
  ;[1 1 1] Set Finish Location
  (set `/Game/TurtlesContent/Blueprints/Character/BP_Turtle.AimLocation` (`self.AimLocation`) _returnvalue)
  ;[1 1 1] Set Nest Location
  (set `/Game/TurtlesContent/Blueprints/Character/BP_Turtle.NestLocation` (`SceneComponent.K2_GetComponentLocation` (`self.Scene`)) _returnvalue)
  ;[1 1 1] Set Behavior Tree for Turtle
  (set `/Game/TurtlesContent/Blueprints/Character/BP_Turtle.BTTurtle` (`self.TurtleBT`) _returnvalue)
  ;[1 1 1] Play effects
  (`self.PlayEffectsOnSpawn`))

(event `PlayEffectsOnSpawn`
  (bind _returnvalue (`SceneComponent.K2_GetComponentLocation` (`self.Scene`)))
  ;[1 1 1] Plays sounds of spawning for creature and for VFX and plays VFX themselves
  (`GameplayStatics.PlaySoundAtLocation` (`self.SpawnSound`) _returnvalue (struct) 1.0 1.0 0.0 null null null)
  (`GameplayStatics.PlaySoundAtLocation` (`self.NestSound`) _returnvalue (struct) 1.0 1.0 0.0 null null null)
  (`|ExecutionSequence`
    (:`then_0`
      (for _array_element (`self.Corners`)
        (bind (_returnvalue_location _returnvalue_rotation _returnvalue_scale) (`KismetMathLibrary.BreakTransform` (`SceneComponent.K2_GetComponentToWorld` _array_element)))
        (`GameplayStatics.SpawnEmitterAtLocation` (`self.SpawnEmitter`) _returnvalue_location _returnvalue_rotation _returnvalue_scale)))
    (:`then_1`
      (`KismetSystemLibrary.Delay` 1.0))))

(fn `UserConstructionScript`)