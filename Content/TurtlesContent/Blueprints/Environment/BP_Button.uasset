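; BP_Button is an environment pressure button that spawns turtles from linked nests.
; On BeginPlay it collects every BP_Nest with its TagName tag and stores raised and lowered positions.
; Any actor overlap plays the Alpha timeline to lerp the button down, and end overlap reverses it.
; The timeline's Finished output calls SpawnTurtle on each linked nest.
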(event `self.ReceiveBeginPlay`
  ;[1 1 1] On begin play - find nests, connected to the button
  (bind _outactors (`GameplayStatics.GetAllActorsOfClassWithTag` "/Game/TurtlesContent/Blueprints/Environment/BP_Nest.BP_Nest_C" (`self.TagName`)))
  (set `self.Nests` _outactors)
  ;[1 1 1] And set two locations for the button
  (bind _output_get (set `self.UnpressedLocation` (`self.K2_GetActorLocation`)))
  (set `self.PressedLocation` (- _output_get (0.0 0.0 8.0))))

(event `self.ReceiveActorBeginOverlap`
  (params (OtherActor :type "Actor Object Reference"))
  ;[1 1 1] The player gets up/leaves the button
  (`self.ButtonPressed`))

(event `self.ReceiveActorEndOverlap`
  (params (OtherActor :type "Actor Object Reference"))
  ;[1 1 1] The player gets up/leaves the button
  (`self.ButtonUnpressed`))

(event `ButtonPressed`
  ;[1 1 1] Change button location
  (bind (_direction _alpha) (`Timeline|Alpha` :!label _label)
    (:`Update`
      (`self.K2_SetActorLocation` (`KismetMathLibrary.VLerp` (`self.UnpressedLocation`) (`self.PressedLocation`) _alpha)))
    (:`Finished`
      ;[1 1 1] Spawn turtle in each connected nest
      (for _array_element (`self.Nests`)
        (bind _asbp_nest (cast `/Game/TurtlesContent/Blueprints/Environment/BP_Nest` _array_element))
        (`/Game/TurtlesContent/Blueprints/Environment/BP_Nest.SpawnTurtle` _asbp_nest)))))

(event `ButtonUnpressed`
  (goto _label :!via `Reverse`))

(fn `UserConstructionScript`)