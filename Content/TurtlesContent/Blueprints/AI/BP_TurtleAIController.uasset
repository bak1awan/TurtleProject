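; AI controller for turtle pawns that starts their behavior tree and seeds its blackboard when possessed.
; After a short delay on possess, it casts the pawn to BP_Turtle and runs the behavior tree stored on that turtle.
; It then sets up BB_Turtle and copies the turtle's aim and nest locations into the blackboard once.
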(event `self.ReceivePossess`
  (params (PossessedPawn :type "Pawn Object Reference"))
  (bind _returnvalue (`AIBlueprintHelperLibrary.GetBlackboard` null))
  (`KismetSystemLibrary.Delay` 0.2)
  (bind _asbp_turtle (cast `/Game/TurtlesContent/Blueprints/Character/BP_Turtle` PossessedPawn))
  ;[1 1 1] Run behavior tree and set variables in blackboard on OnPossess event
  (`self.RunBehaviorTree` (`/Game/TurtlesContent/Blueprints/Character/BP_Turtle.BTTurtle` _asbp_turtle))
  (`self.UseBlackboard` "/Game/TurtlesContent/Blueprints/AI/BB_Turtle.BB_Turtle")
  (`BlackboardComponent.SetValueAsVector` _returnvalue "AimLocation" (`/Game/TurtlesContent/Blueprints/Character/BP_Turtle.AimLocation` _asbp_turtle))
  (`BlackboardComponent.SetValueAsVector` _returnvalue "NestLocation" (`/Game/TurtlesContent/Blueprints/Character/BP_Turtle.NestLocation` _asbp_turtle)))

(fn `UserConstructionScript`)